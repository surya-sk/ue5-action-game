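; Bird call ambience Blueprint that plays sounds from random actors during the day and halts them at night.
; On BeginPlay it finds the BP_TimeOfDay actor and binds to its dusk and morning events.
; Dusk clears the continue-playing flag and unbinds the current actor's audio-finished event, breaking the chain.
; Morning sets the flag and restarts random playback, while sound-finished handling defers to the parent class.
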(event `self.ReceiveBeginPlay`
  ;[1 1 1] Find the Time of Day actor, and bind our start and stop events to dusk and morning
  (bind _returnvalue (`GameplayStatics.GetActorOfClass` "/Game/Blueprints/BP_TimeOfDay.BP_TimeOfDay_C"))
  (bind _output_get (set `self.TimeOfDayBlueprint` _returnvalue))
  (`/Engine/EditorBlueprintResources/StandardMacros.IsValid` _output_get
    (:`Is Valid`
      (add `/Game/Blueprints/BP_TimeOfDay.Dusk` _output_get (delegate `HaltSoundsAtNight`))
      (add `/Game/Blueprints/BP_TimeOfDay.Morning` _output_get (delegate `BeginSoundsAtMorning`)))))

(event `HaltSoundsAtNight`
  (bind _currentplayingactor (`self.CurrentPlayingActor`))
  ;[1 1 1] At night, make sure we stop playing sounds
  (set `self.ShouldContinuePlaying` false)
  (`/Engine/EditorBlueprintResources/StandardMacros.IsValid` _currentplayingactor
    (:`Is Valid`
      (remove `/Game/Audio/AudioBlueprints/BP_AudioActor_RandomAmb.AudioFinished` _currentplayingactor (delegate `self.OnSoundFinished`)))))

(event `self.OnSoundFinished`
  ;[1 1 1] At night, make sure we stop playing sounds
  (`parent.OnSoundFinished`))

(event `BeginSoundsAtMorning`
  ;[1 1 1] In the morning, kick off the process all over again
  (set `self.ShouldContinuePlaying` true)
  (`self.PlaySoundFromRandomActor`))

(fn `UserConstructionScript`)