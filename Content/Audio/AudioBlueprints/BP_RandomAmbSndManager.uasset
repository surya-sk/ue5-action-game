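; Manager actor that plays intermittent random ambient sounds from a list of sound actors.
; On BeginPlay it waits a random delay within a min/max range, then picks a random actor and starts its sound.
; It binds to that actor's audio-finished event, which unbinds and restarts the delay, looping while ShouldContinuePlaying is true.
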(event `self.ReceiveBeginPlay`
  ;[1 1 1] Kick off the process at the end
  (`self.OnSoundFinished`))

(event `PlaySoundFromRandomActor`
  ;[1 1 1] Pick a random actor from our list, and bind our Audio Finished event to the random actor's finished even
  (bind _output_get (set `self.CurrentPlayingActor` (`KismetArrayLibrary.Array_Random` (`self.RandomSoundActors`))))
  (`/Game/Audio/AudioBlueprints/BP_AudioActor_AmbientSoundModulator.StartPlayingSound` _output_get)
  (add `/Game/Audio/AudioBlueprints/BP_AudioActor_RandomAmb.AudioFinished` _output_get (delegate `OnSoundFinished`)))

(event `OnSoundFinished`
  (bind _currentplayingactor (`self.CurrentPlayingActor`))
  ;[1 1 1] When a sound has finished playing, unbind the finished event in case something goes wrong, then wait a random amount of time to fire a new sound
  (`/Engine/EditorBlueprintResources/StandardMacros.IsValid` _currentplayingactor
    (:`Is Valid`
      (remove `/Game/Audio/AudioBlueprints/BP_AudioActor_RandomAmb.AudioFinished` _currentplayingactor (delegate `OnSoundFinished`)))
    (:`Is Not Valid`
      _))
  (`KismetSystemLibrary.RetriggerableDelay` (`KismetMathLibrary.RandomFloatInRange` (`self.MinResetTime`) (`self.MaxResetTime`)))
  (if (`self.ShouldContinuePlaying`)
    (`self.PlaySoundFromRandomActor`)))

(fn `UserConstructionScript`)