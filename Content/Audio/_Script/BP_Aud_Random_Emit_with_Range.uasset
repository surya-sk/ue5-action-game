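; Audio emitter actor that repeatedly plays a sound at random positions around itself.
; From BeginPlay it waits a random time between minimum and maximum settings, then plays the sound at its location plus an offset from CreateRandomLocation.
; Offsets scale with MaxDistRange, with Z intended to stay at or above the actor.
; OnAudioFinished restarts the loop after a short fixed delay, independent of actual playback completion.
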(event `self.ReceiveBeginPlay`
  (`KismetSystemLibrary.Delay` (`KismetMathLibrary.RandomFloatInRange` (`self.WaitTimeMin`) (`self.WaitTimeMAx`)) :!label _label)
  (`GameplayStatics.PlaySoundAtLocation` (`self.Sound`) (+ (`self.K2_GetActorLocation` self) (`KismetMathLibrary.MakeVector` (* (`KismetMathLibrary.RandomFloatInRange` 0.0 (`self.MaxDistRange`)) (`KismetMathLibrary.RandomFloatInRange` -1.0 1.0)) (* (`KismetMathLibrary.RandomFloatInRange` 0.0 (`self.MaxDistRange`)) (`KismetMathLibrary.RandomFloatInRange` -1.0 1.0)) (`KismetMathLibrary.RandomFloatInRange` 0.0 (`self.MaxDistRange`)))) (struct) 1.0 1.0 0.0 null null null)
  (`KismetSystemLibrary.Delay` 0.2)
  (`self.OnAudioFinished`))

(event `OnAudioFinished`
  (goto _label))

(fn `UserConstructionScript`)