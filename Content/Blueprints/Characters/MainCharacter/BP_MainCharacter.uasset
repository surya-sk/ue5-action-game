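; Player character that can mount and ride a horse, with switchable third-person and first-person views.
; Rider events let the horse drive mounting, dismounting and re-possession, with Timelines blending actor and camera transforms for smooth handovers.
; Mounting and stirrup leg IK relay through authority checks to the AnimBP.
; FPS mode attaches the boom to a head-follow socket, with per-tick pitch clamping; debug-style keys save and load.
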(event `self.ReceiveBeginPlay`
  (`self.Begin Play Ref setup`))

(event `self.ReceiveTick`
  (params (DeltaSeconds :type "Float (single-precision)"))
  (`self.Tick Events`))

(event `Tick Events`
  ;[0 0.5558 1 1 50] Reference setup
  ;;[1 1 1] Connect [tick events] to your tick if trasnfering this blueprint to a different class
  (`self.FPS camera rotation limits and breakup correction`)
  (`self.Stirrup IK Correction`))

(event `/Game/UltimateHorsePack/Blueprints/BPI_HorseRiding.Rider Set Replicated Movement`
  (params (Replicated :type Boolean))
  ;[1 1 1 1 44] Movement Replication Toggle
  (`self.SetReplicateMovement` Replicated))

(event `/Game/UltimateHorsePack/Blueprints/BPI_HorseRiding.Rider Update Horse Reference`
  (params (Horse :type "/Game/UltimateHorsePack/Blueprints/BP_Horse Object Reference"))
  ;[0 0.5558 1 1 50] Reference setup
  (`/Engine/EditorBlueprintResources/StandardMacros.IsValid` (`self.HorseRef`)
    (:`Is Not Valid`
      (set `self.HorseRef` Horse))))

(event `Begin Play Ref setup`
  ;[0 0.5558 1 1 50] Reference setup
  (set `self.ABP` (`SkeletalMeshComponent.GetAnimInstance` (`self.Mesh`)))
  (set `self.bHatEquiped` false)
  ;[1 1 1] UE 5.1.0  New Input mapping initialization
  (bind _asplayer_controller (cast `PlayerController` (`self.GetController`)))
  (`EnhancedInputSubsystemInterface.AddMappingContext` (pcsubsystem `EnhancedInputLocalPlayerSubsystem` _asplayer_controller) "/Game/UltimateHorsePack/Blueprints/InputMappingsPS4.InputMappingsPS4" 0 (struct)))

(event `EnhancedInput|/Game/UltimateHorsePack/Blueprints/InputAction_Mount`
  (params (ActionValue :type Boolean) (ElapsedSeconds :type "Float (double-precision)") (TriggeredSeconds :type "Float (double-precision)") (InputAction :type "InputAction Object Reference" :default "/Game/UltimateHorsePack/Blueprints/InputAction_Mount.InputAction_Mount"))
  ;[0.03277 1 0] Attempt to Mount the horse
  (:`Started`
    (set `self.FPS_HorseRef` (`self.HorseRef`))
    (`self.Attempt to mount the horse`)))

(event `/Game/UltimateHorsePack/Blueprints/BPI_HorseRiding.Rider Clear Horse Reference`
  ;[0 0.5558 1 1 50] Reference setup
  (`/Engine/EditorBlueprintResources/StandardMacros.IsValid` (`self.HorseRef`)
    (:`Is Valid`
      (set `self.HorseRef` null))))

(event `Attempt to mount the horse`
  (bind _horseref (`self.HorseRef`))
  ;[0.03277 1 0] Attempt to Mount the horse
  (`/Engine/EditorBlueprintResources/StandardMacros.IsValid` _horseref
    (:`Is Valid`
      (`/Game/UltimateHorsePack/Blueprints/BP_Horse.Rider Attempt Mounting` _horseref)
      (`/Engine/EditorBlueprintResources/ActorMacros.Switch Has Authority`
        (:`Remote`
          (`self.Client Attempt to Mount`))))))

(event `Server IK update`
  (params (MountedLegIk_Alpha :type "Float (single-precision)"))
  ;[1 0.7278 0] Replication code for Riders Feet IK while horse Riding
  (`self.Set IK value` MountedLegIk_Alpha)
  (`/Engine/EditorBlueprintResources/ActorMacros.Switch Has Authority`
    (:`Remote`
      (`self.Client IK update` MountedLegIk_Alpha))))

(event `Client Attempt to Mount`
  (bind _horseref (`self.HorseRef`))
  ;[0.03277 1 0] Attempt to Mount the horse
  (`/Engine/EditorBlueprintResources/StandardMacros.IsValid` _horseref
    (:`Is Valid`
      (`/Game/UltimateHorsePack/Blueprints/BP_Horse.Rider Attempt Mounting` _horseref))))

(event `/Game/UltimateHorsePack/Blueprints/BPI_HorseRiding.Rider Match Camera to Horse Actor`
  (params (`Horse Ref` :type "/Game/UltimateHorsePack/Blueprints/BP_Horse Object Reference"))
  (bind _followcamera (`self.FollowCamera`))
  ;[1 0.6991 0 1 45] SYNC character location to horse for smooother mount sequence
  (bind _output_get (set `self.HorseRef` `Horse Ref`))
  (if (`self.FPS mode`)
    _
    (else
      _))
  (set `self.PauseInput` true)
  (bind (_direction _alpha) (`Timeline|Timeline` :!via `PlayFromStart`)
    (:`Update`
      (`self.FollowCamera`
        (:`then`
          (`SceneComponent.K2_SetWorldTransform` _followcamera (`KismetMathLibrary.TLerp` (`SceneComponent.K2_GetComponentToWorld` _followcamera) (`SceneComponent.K2_GetComponentToWorld` (`/Game/UltimateHorsePack/Blueprints/BP_Horse.Camera` _output_get)) _alpha "DualQuatInterp") false true))
        (:`else`)))
    (:`Finished`
      (set `self.PauseInput` false)
      (set `self.PauseCameraInput` false))))

(event `Set IK value`
  (params (MountedLegIk_Alpha :type "Float (single-precision)"))
  ;[1 0.7278 0] Replication code for Riders Feet IK while horse Riding
  (message `/Game/UltimateHorsePack/Blueprints/BPI_RiderABP_control.Update Leg IK` (`self.ABP`) MountedLegIk_Alpha))

(event `Client IK update`
  (params (MountedLegIk_Alpha :type "Float (single-precision)"))
  ;[1 0.7278 0] Replication code for Riders Feet IK while horse Riding
  (`self.Set IK value` MountedLegIk_Alpha))

(event `/Game/UltimateHorsePack/Blueprints/BPI_HorseRiding.Rider Server IK update`
  (params (`IK alpha` :type "Float (double-precision)"))
  ;[1 0.7278 0] Replication code for Riders Feet IK while horse Riding
  (`self.Server IK update` `IK alpha`))

(event `/Game/UltimateHorsePack/Blueprints/BPI_HorseRiding.Rider Sync Location`
  (params (Dismount :type Boolean) (NewTransform :type "Transform Structure"))
  ;[1 0.6991 0 1 45] SYNC character location to horse for smooother mount sequence
  (set `self.Temp_Transform` (`self.GetTransform`))
  (`PrimitiveComponent.SetCollisionEnabled` (`self.CapsuleComponent`) "NoCollision")
  (set `SpringArmComponent.bDoCollisionTest` false (`self.CameraBoom`))
  (if Dismount
    (bind (_direction _alpha) (`Timeline|Timeline_1` :!via `PlayFromStart`)
      (:`Update`
        (`self.K2_SetActorTransform` (`KismetMathLibrary.TLerp` (`self.Temp_Transform`) (`KismetMathLibrary.MakeTransform` (+ (.location NewTransform) (0.0 0.0 50.0)) (.rotation NewTransform)) _alpha "EulerInterp") false true))
      (:`Finished`
        (message `/Game/UltimateHorsePack/Blueprints/BPI_RiderABP_control.Update Horse Mode` (`self.ABP`) false)
        (`PrimitiveComponent.SetCollisionEnabled` (`self.CapsuleComponent`) "QueryAndPhysics")
        ;[1 0.7278 0] Replication code for Riders Feet IK while horse Riding
        (`self.SetHorseState` self false)
        (`KismetSystemLibrary.PrintString` "Dismounted")))
    (else
      (bind (_direction_2 _alpha_2) (`Timeline|Timeline_0` :!via `PlayFromStart`)
        (:`Update`
          (`self.K2_SetActorTransform` (`KismetMathLibrary.TLerp` (`self.Temp_Transform`) (`KismetMathLibrary.MakeTransform` (.location NewTransform) (.rotation NewTransform)) _alpha_2 "EulerInterp") false true))
        (:`Finished`
          (`self.SetHorseState` self true))))))

(event `Switch to FPS mode`
  (bind _returnvalue (`self.GetController`))
  ;[0.0356 0.4072 0 1 70] FPS mode
  (set `self.PauseInput` false)
  (`/Engine/EditorBlueprintResources/StandardMacros.IsValid` _returnvalue
    (:`Is Valid`
      (`Controller.SetControlRotation` _returnvalue (`SpringArmComponent.GetTargetRotation` (`self.CameraBoom`))))
    (:`Is Not Valid`
      _))
  (set `SpringArmComponent.bUsePawnControlRotation` true (`self.CameraBoom`))
  (set `CharacterMovementComponent.RotationRate` (struct :`Yaw` 99999.0) (`self.CharacterMovement`))
  (set `self.bUseControllerRotationYaw` true)
  (set `CharacterMovementComponent.bOrientRotationToMovement` false (`self.CharacterMovement`))
  (set `self.FPS mode` true))

(event `/Game/UltimateHorsePack/Blueprints/BPI_HorseRiding.Rider Set  Hat Equiped`
  (params (HatEquipped :type Boolean))
  ;[1 0.7278 0] Replication code for Riders Feet IK while horse Riding
  (set `self.bHatEquiped` HatEquipped))

(event `/Game/UltimateHorsePack/Blueprints/BPI_HorseRiding.Rider Set Max Move Speed`
  (params (Speed :type "Float (double-precision)"))
  ;[1 0.7278 0] Replication code for Riders Feet IK while horse Riding
  (set `CharacterMovementComponent.MaxWalkSpeed` Speed (`self.CharacterMovement`)))

(event `Disable FPS mode`
  (bind _cameraboom (`self.CameraBoom`))
  ;[0.0356 0.4072 0 1 70] FPS mode
  (set `self.PauseInput` false)
  (set `SpringArmComponent.TargetArmLength` 400.0 (`self.CameraBoom`))
  (set `SpringArmComponent.bUsePawnControlRotation` true (`self.CameraBoom`))
  (`SceneComponent.K2_SetRelativeLocation` _cameraboom (4.0 0.0 3.0) false true)
  (`SceneComponent.ResetRelativeTransform` _cameraboom)
  (set `self.FPS mode` false)
  (message `/Game/UltimateHorsePack/Blueprints/BPI_RiderABP_control.Update FPS body Rotation` (`self.ABP`) (struct))
  (set `CharacterMovementComponent.RotationRate` (struct :`Yaw` 500.0) (`self.CharacterMovement`))
  (set `self.bUseControllerRotationYaw` false)
  (set `CharacterMovementComponent.bOrientRotationToMovement` true (`self.CharacterMovement`))
  (`SceneComponent.ResetRelativeTransform` (`self.FollowCamera`)))

(event `/Game/UltimateHorsePack/Blueprints/BPI_HorseRiding.Rider Dismounted - Sync camera back to Rider`
  (bind _followcamera (`self.FollowCamera`))
  ;[0.1552 1 0 1 44] Switchg Camera from Horse to Rider (happens during pawn re-possesion)
  (set `self.PauseInput` true)
  (bind (_direction _alpha) (`Timeline|Timeline_2` :!via `PlayFromStart`)
    (:`Update`
      (`SceneComponent.K2_SetRelativeTransform` _followcamera (`KismetMathLibrary.TLerp` (`SceneComponent.GetRelativeTransform` _followcamera) (`KismetMathLibrary.MakeTransform` (0.0 0.0 0.0)) _alpha "DualQuatInterp") false false))
    (:`Finished`
      (set `self.PauseInput` false)
      (set `self.PauseCameraInput` false))))

(event `/Game/UltimateHorsePack/Blueprints/BPI_HorseRiding.Rider Set Actor Loc and Rot`
  (params (Loc :type "Vector Structure") (Rot :type "Rotator Structure"))
  ;[0.06646 1 0 1 44] Actor Location Update
  (`self.K2_SetActorLocationAndRotation` Loc Rot false true))

(event `/Game/UltimateHorsePack/Blueprints/BPI_HorseRiding.Rider Set Actor Loc`
  (params (newLoc :type "Vector Structure"))
  ;[0.06646 1 0 1 44] Actor Location Update
  (`self.K2_SetActorLocation` newLoc true))

(event `/Game/UltimateHorsePack/Blueprints/BPI_HorseRiding.Rider Load FPS mode`
  (bind _cameraboom (`self.CameraBoom`))
  ;[0.0356 0.4072 0 1 70] FPS mode
  (set `self.FPS mode` true)
  (message `/Game/UltimateHorsePack/Blueprints/BPI_RiderABP_control.Update FPS mode` (`self.ABP`) true)
  (set `self.LoadingFPS` true)
  (set `self.PauseInput` true)
  (`SceneComponent.K2_AttachToComponent` (`self.CameraBoom`) (`self.Mesh`) "FPS_Socket" "SnapToTarget" "KeepWorld" "KeepRelative" true)
  (set `SpringArmComponent.TargetArmLength` 0.0 _cameraboom)
  (set `SpringArmComponent.bUsePawnControlRotation` false _cameraboom)
  (`self.Switch to FPS mode`))

(event `/Game/UltimateHorsePack/Blueprints/BPI_HorseRiding.Rider Pause Input`
  (params (Pause :type Boolean))
  ;[0.1552 1 0 1 44] Switchg Camera from Horse to Rider (happens during pawn re-possesion)
  (bind _output_get (set `self.PauseInput` Pause))
  (set `self.PauseCameraInput` _output_get))

(event `/Game/UltimateHorsePack/Blueprints/BPI_HorseRiding.Rider Re-enable Character`
  (params (NewController :type "Controller Object Reference"))
  ;[0.08738 1 0 1 40] dismounting the horse > Re-posses character
  (`|ExecutionSequence`
    (:`then_0`
      (set `self.CurrentController` NewController))
    (:`then_1`
      (`/Engine/EditorBlueprintResources/ActorMacros.Switch Has Authority`
        (:`Authority`
          (`Controller.Possess` NewController self)
          (`self.SetReplicateMovement` true))
        (:`Remote`
          _))
      (`PrimitiveComponent.SetCollisionEnabled` (`self.CapsuleComponent`) "QueryAndPhysics")
      (`SceneComponent.K2_SetRelativeLocationAndRotation` :`self` (`self.FollowCamera`) :`bTeleport` true)
      (set `self.PauseInput` false)
      (set `CharacterMovementComponent.MaxWalkSpeed` 500.0 (`self.CharacterMovement`))
      (`KismetSystemLibrary.Delay` 1.0)
      (set `SpringArmComponent.bDoCollisionTest` true (`self.CameraBoom`))
      (message `/Game/UltimateHorsePack/Blueprints/BPI_RiderABP_control.Update Mounted Leg IK` (`self.ABP`) 0.0)
      (`SceneComponent.ResetRelativeTransform` (`self.FollowCamera`))
      (set `self.HorseRef` null)
      (set `self.FPS_HorseRef` null)
      (`/Engine/EditorBlueprintResources/ActorMacros.Switch Has Authority`
        (:`Remote`
          (`PrimitiveComponent.SetCollisionEnabled` (`self.CapsuleComponent`) "QueryAndPhysics"))))))

(event `/Game/UltimateHorsePack/Blueprints/BPI_HorseRiding.Rider Set FPS horse Mode`
  (params (`FPS mode` :type Boolean))
  ;[0.0356 0.4072 0 1 70] FPS mode
  (set `self.FPS mode` `FPS mode`))

(event `/Game/UltimateHorsePack/Blueprints/BPI_HorseRiding.Rider Unload FPS mode`
  (bind _abp (`self.ABP`))
  ;[0.0356 0.4072 0 1 70] FPS mode
  (message `/Game/UltimateHorsePack/Blueprints/BPI_RiderABP_control.Update FPS mode` _abp false)
  (set `self.LoadingFPS` false)
  (set `self.PauseInput` true)
  (`SceneComponent.K2_AttachToComponent` (`self.CameraBoom`) (`self.CapsuleComponent`) "None" "SnapToTarget" "SnapToTarget" "KeepRelative" true)
  (`SceneComponent.ResetRelativeTransform` (`self.CameraBoom`))
  (`self.Disable FPS mode`)
  (message `/Game/UltimateHorsePack/Blueprints/BPI_RiderABP_control.Update Input Axis` _abp 1.0))

(event `/Game/UltimateHorsePack/Blueprints/BPI_HorseRiding.Rider Update Horse FPS mode`
  (params (`Horse FPS mode` :type Boolean))
  ;[0.0356 0.4072 0 1 70] FPS mode
  (set `self.FPS_HorseMode` `Horse FPS mode`))

(event `Key|S`
  (params (Key :type "Key Structure"))
  (:`Pressed`
    (`self.SaveGame`)))

(event `Key|M`
  (params (Key :type "Key Structure"))
  (:`Pressed`
    (`self.LoadGame`)))

(fn `FPS camera rotation limits and breakup correction`
  (bind _followcamera (`self.FollowCamera`))
  (bind _followcamera_2 (`self.FollowCamera`))
  (bind (_returnvalue_roll _returnvalue_pitch _returnvalue_yaw) (`KismetMathLibrary.BreakRotator` (`SceneComponent.K2_GetComponentRotation` (`self.FollowCamera`))))
  (bind (_relativerotation_roll _relativerotation_pitch _relativerotation_yaw) (`KismetMathLibrary.BreakRotator` (`SceneComponent.RelativeRotation` _followcamera)))
  (if (`self.FPS mode`)
    (if (< _returnvalue_pitch -70.0)
      (`SceneComponent.K2_SetWorldRotation` _followcamera_2 (`KismetMathLibrary.MakeRotator` 0.0 -70.0 _returnvalue_yaw) false false)
      (elif (> _returnvalue_pitch 40.0)
        (`SceneComponent.K2_SetWorldRotation` _followcamera_2 (`KismetMathLibrary.MakeRotator` 0.0 40.0 _returnvalue_yaw) false false)
        (elif (or (`KismetMathLibrary.NearlyEqual_FloatFloat` _relativerotation_yaw 180.0 5.0) (`KismetMathLibrary.NearlyEqual_FloatFloat` _relativerotation_yaw -180.0 5.0))
          (`SceneComponent.K2_SetWorldRotation` :`self` _followcamera)
          (`SceneComponent.K2_SetRelativeRotation` :`self` _followcamera))))))

(fn `Get IF actor can be a Rider`
  (returns (Rider :type Boolean))
  (return true))

(fn `Get Rider ABP`
  (returns (ABP :type "AnimInstance Object Reference"))
  (return (`SkeletalMeshComponent.GetAnimInstance` (`self.Mesh`))))

(fn `Get Rider Actor Loc and Rot`
  (returns (Loc :type "Vector Structure") (Rot :type "Rotator Structure"))
  (return (`self.K2_GetActorLocation`) (`self.K2_GetActorRotation`)))

(fn `Get Rider Controller`
  (returns (Output :type "Controller Object Reference"))
  (return (`self.GetController`)))

(fn `Get Rider FPS mode value`
  (returns (`FPS mode` :type Boolean))
  (return (`self.FPS mode`)))

(fn `Get Rider Mesh`
  (returns (Mesh :type "SkeletalMeshComponent Object Reference"))
  (return (`self.Mesh`)))

(fn `Get Riders Player Controller`
  (returns (Output :type "PlayerController Object Reference"))
  (return (`self.GetLocalViewingPlayerController`)))

(fn `Is Riders Hat Equiped`
  (returns (` HatEquiped` :type Boolean))
  (return (`self.bHatEquiped`)))

(fn `Stirrup IK Correction`
  (if (`NavMovementComponent.IsFalling` (`self.CharacterMovement`))
    (message `/Game/UltimateHorsePack/Blueprints/BPI_RiderABP_control.Update Mounted Leg IK` (`self.ABP`) 0.0)))

(fn `UserConstructionScript`)